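; BP_Stairs is an interactable staircase that rotates when a "Door" item enters its box.
; A matching BP_UsableItemChild unlocks an achievement with a narrator line on the main character, found at BeginPlay.
; A timeline then lerps the stairs' world rotation and destroys the item on finish.
; DoOnce precedes the item check, so the first overlap by any actor uses up the trigger.
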(event OnComponentBeginOverlap(Box)
  (params (OverlappedComponent :type Primitive%20Component%20Object%20Reference) (OtherActor :type Actor%20Object%20Reference) (OtherComp :type Primitive%20Component%20Object%20Reference) (OtherBodyIndex :type Integer) (bFromSweep :type Boolean) (SweepResult :type Hit%20Result%20Structure%20%28by%20ref%29))
  (Utilities|FlowControl|DoOnce false
    (:Completed
      (bind _asbp_usable_item_child (Utilities|Casting|CastToBP_UsableItemChild OtherActor))
      (if (Utilities|Enum|Equal(Enum) (.description (Variables|/Game/Blueprints/Inventory/BP_MasterPickUpItem.BP_MasterPickUpItem_C|GetItemData _asbp_usable_item_child)) (Variables|Default|GetDoor))
        (Default|UnlockAchievement (Variables|Default|GetPlayerRef) "3" "Pyro")
        (bind _alpha (Timeline|TL_RotatingStairs PlayFromStart)
          (:Update
            (Transformation|SetWorldRotation (Variables|Default|GetStairs) (Math|Rotator|Lerp(Rotator) "40.000000,0.000000,0.000000" "0, 0, 0" _alpha true) false false))
          (:Finished
            (Actor|DestroyActor OtherActor)))))))

(event EventBeginPlay
  (bind _outactors (Actor|GetAllActorsOfClass "/Game/Blueprints/BP_MainCharacter.BP_MainCharacter_C"))
  (Variables|Default|SetPlayerRef (Utilities|Array|Get(acopy) _outactors)))

(fn ConstructionScript)