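; BP_WaterPool is an interactable trigger that fills with rising water when a bottle item enters its box.
; It caches the main character at BeginPlay and, on a bottle overlap, unlocks an achievement with a narrator line on that player.
; A timeline lerps the water's relative position upward, then destroys the bottle.
; A DoOnce precedes the item check, so the first overlap of any actor uses up the trigger.
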(event OnComponentBeginOverlap(Box)
  (params (OverlappedComponent :type Primitive%20Component%20Object%20Reference) (OtherActor :type Actor%20Object%20Reference) (OtherComp :type Primitive%20Component%20Object%20Reference) (OtherBodyIndex :type Integer) (bFromSweep :type Boolean) (SweepResult :type Hit%20Result%20Structure%20%28by%20ref%29))
  (Utilities|FlowControl|DoOnce false
    (:Completed
      (bind _asbp_usable_item_child (Utilities|Casting|CastToBP_UsableItemChild OtherActor))
      (if (Utilities|Enum|Equal(Enum) (.description (Variables|/Game/Blueprints/Inventory/BP_MasterPickUpItem.BP_MasterPickUpItem_C|GetItemData _asbp_usable_item_child)) (Variables|Default|GetBottle))
        (Default|UnlockAchievement (Variables|Default|GetPlayerRef) "5" "Pyro")
        (bind _alpha (Timeline|TL_WaterPosition PlayFromStart)
          (:Update
            (Transformation|SetRelativeLocation (Variables|Default|GetWater) (Math|Vector|Lerp(Vector) "0.000000,0.000000,-85.000000" "0.000000,0.000000,180.000000" _alpha) false false))
          (:Finished
            (Actor|DestroyActor OtherActor)))))))

(event EventBeginPlay
  (bind _outactors (Actor|GetAllActorsOfClass "/Game/Blueprints/BP_MainCharacter.BP_MainCharacter_C"))
  (Variables|Default|SetPlayerRef (Utilities|Array|Get(acopy) _outactors)))

(fn ConstructionScript)