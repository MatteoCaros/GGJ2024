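; BP_RedButton is a one-shot interactable red button that unlocks an achievement and spawns a giant cat.
; The first Interact call triggers the achievement on the main character, plays a boom sound and runs a timeline that lerps the button mesh down.
; When the press finishes, it spawns a scaled-up BP_Cat at an offset from the actor and plays a purr sound.
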(event EventInteract
  (params (MainCharacterRef :type BP%20Main%20Character%20Object%20Reference))
  (bind _button (Variables|Default|GetButton))
  (bind _relativelocation (Variables|/Script/Engine.SceneComponent|GetRelativeLocation _button))
  (Utilities|FlowControl|DoOnce false
    (:Completed
      (Default|UnlockAchievement MainCharacterRef "2" "None")
      (Audio|PlaySound2D "/Game/Audio/RandomFunnySounds/BOOM.BOOM" 1.0 1.0 0.0 0 0)
      (bind _alpha (Timeline|TMLPressButton PlayFromStart)
        (:Update
          (Transformation|SetRelativeLocation (Variables|Default|GetButton) (Math|Vector|MakeVector (.x _relativelocation) (.y _relativelocation) (Math|Float|Lerp 0.0 -25.0 _alpha)) false false))
        (:Finished
          (Game|SpawnActorfromClass "/Game/Blueprints/Inventory/UsableItem/BP_Cat.BP_Cat_C" (Math|Transform|MakeTransform (+ (Variables|Default|GetSpawnCatLocation) (Transformation|GetActorLocation)) "0, 0, 0" "5.000000,5.000000,5.000000") "AlwaysSpawn" "MultiplyWithRoot" 0 0)
          (Audio|PlaySound2D "/Game/Audio/SFXs/SFX_Cat_Purr.SFX_Cat_Purr" 1.0 1.0 0.0 0 0))))))

(fn ConstructionScript)