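; BP_Door is an interactable hinged door that a Player-tagged character toggles open and closed.
; Interact passes through a FlipFlop to Open or Close, with a ClockWise flag choosing the swing direction before opening.
; Both play a sound and drive one timeline forward or in reverse to lerp the mesh's relative rotation.
; CanBeOpened blocks further interaction until the timeline finishes.
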(event Custom|Close
  (Variables|Default|SetCanBeOpened false)
  (Audio|PlaySound2D "/Game/Audio/SFXs/SFX_Inside_Door_Close.SFX_Inside_Door_Close" 1.0 1.0 0.0 0 0)
  (bind _alpha (Timeline|Door_Rotation Reverse)
    (:Update
      (Transformation|SetRelativeRotation (Variables|Default|GetStaticMesh) (Math|Rotator|Lerp(Rotator) (Variables|Default|GetStartRot) (Variables|Default|GetEndRot) _alpha true) false false))
    (:Finished
      (Variables|Default|SetCanBeOpened true))))

(event Custom|Open
  (Variables|Default|SetCanBeOpened false)
  (Audio|PlaySound2D "/Game/Audio/SFXs/SFX_Inside_Door_Open.SFX_Inside_Door_Open" 1.0 1.0 0.0 0 0)
  (bind _alpha (Timeline|Door_Rotation Play)
    (:Update
      (Transformation|SetRelativeRotation (Variables|Default|GetStaticMesh) (Math|Rotator|Lerp(Rotator) (Variables|Default|GetStartRot) (Variables|Default|GetEndRot) _alpha true) false false))
    (:Finished
      (Variables|Default|SetCanBeOpened true))))

(event EventInteract
  (params (MainCharacterRef :type BP%20Main%20Character%20Object%20Reference))
  (if (Variables|Default|GetCanBeOpened)
    (if (Actor|ActorHasTag MainCharacterRef "Player")
      (Utilities|FlowControl|FlipFlop
        (:A
          (if (Variables|Default|GetClockWise?)
            (Variables|Default|SetEndRot "0.000000,120.000000,0.000000")
            (else
              (Variables|Default|SetEndRot "0.000000,-120.000000,0.000000")))
          (CallFunction|Open))
        (:B
          (CallFunction|Close))))))

(fn ConstructionScript)