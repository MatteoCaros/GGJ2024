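; BP_TelevisionMonitor is an interactable television that toggles a Gandalf video and its song on and off.
; BeginPlay starts the song, immediately pauses it, and opens the Gandalf source on the media player.
; Interact uses a FlipFlop to swap the monitor material between video and off while unpausing or pausing the song.
; The media player itself is never paused, only hidden by the material swap.
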(event EventInteract
  (params (MainCharacterRef :type BP%20Main%20Character%20Object%20Reference))
  (bind _monitor (Variables|Default|GetMonitor))
  (bind _song (Variables|Default|GetSong))
  (Utilities|FlowControl|FlipFlop
    (:A
      (Rendering|Material|SetMaterial _monitor 0 "/Game/Movies/GandalfPlayer_video_Mat.GandalfPlayer_video_Mat")
      (Class|AudioComponent|SetPaused _song false))
    (:B
      (Rendering|Material|SetMaterial _monitor 0 "/Game/Movies/Television_Off.Television_Off")
      (Class|AudioComponent|SetPaused _song true))))

(event EventBeginPlay
  (bind _song (Variables|Default|GetSong))
  (Audio|Components|Audio|Play _song 0.0)
  (Class|AudioComponent|SetPaused _song true)
  (Media|MediaPlayer|OpenSource (Variables|Default|GetMediaPlayer) "/Game/Movies/Gandalf.Gandalf"))

(fn ConstructionScript)