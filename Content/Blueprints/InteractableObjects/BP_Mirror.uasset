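; BP_Mirror is an interactable mirror that triggers an end-of-game sequence.
; Its first Interact disables player input, unlocks an achievement with a narrator line, and queues "Supercazzola" audio on the character's subtitle manager.
; When the subtitle manager finishes reading all lines, a bound EndGame event fades camera and audio out, then opens the level referenced by Map.
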(event Custom|EndGame
  (CameraFades|StartCameraFade :self (Game|GetPlayerCameraManager 0) :ToAlpha 1.0 :Duration 4.0 :bShouldFadeAudio true)
  (Utilities|FlowControl|Delay 4.0)
  (Game|OpenLevel(byObjectReference) "/Game/Levels/Map.Map"))

(event EventInteract
  (params (MainCharacterRef :type BP%20Main%20Character%20Object%20Reference))
  (bind _subtitle_manager_ref (Variables|/Game/Blueprints/BP_MainCharacter.BP_MainCharacter_C|GetSubtitle%20Manager%20Ref MainCharacterRef))
  (Utilities|FlowControl|DoOnce false
    (:Completed
      (Input|DisableInput MainCharacterRef 0)
      (Default|UnlockAchievement MainCharacterRef "7" "GGJ_VO_A_volte_le_cose_si_scoprono_per_caso")
      (Default|AddAudiotoPlay _subtitle_manager_ref "Supercazzola")
      (EventDispatchers|BindEventtoOnEndReadAlllines _subtitle_manager_ref (delegate Custom|EndGame)))))

(fn ConstructionScript)