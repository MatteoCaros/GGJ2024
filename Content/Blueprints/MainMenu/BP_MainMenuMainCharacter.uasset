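; BP_MainMenuMainCharacter is the temporary main menu pawn that hands control to the gameplay character once the intro finishes.
; On BeginPlay it shows WB_MainMenu with the mouse cursor and binds the widget's Play click to start the IntroSequencer level sequence.
; When the sequence finishes, it possesses MainPlayer, removes the sequencer and menu, switches to game-only input and destroys itself.
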(event Custom|StartPlayAnimation
  (Sequencer|Player|Play (Variables|/Script/LevelSequence.LevelSequenceActor|GetSequencePlayer (Variables|Default|GetIntroSequencer)) :!class /Script/MovieScene.MovieSceneSequencePlayer))

(event Custom|OnFinishPlayAnimation
  (bind _returnvalue (Game|GetPlayerController 0))
  (Pawn|Possess (Game|GetPlayerController 0) (Variables|Default|GetMainPlayer))
  (Actor|DestroyActor (Variables|Default|GetIntroSequencer))
  (Widget|RemovefromParent (Variables|Default|GetMainMenuWidget))
  (Variables|/Script/Engine.PlayerController|SetbShowMouseCursor _returnvalue false)
  (Input|SetInputModeGameOnly _returnvalue false)
  (Actor|DestroyActor))

(event EventBeginPlay
  (bind _returnvalue (Pawn|GetController))
  (bind _asplayer_controller (Utilities|Casting|CastToPlayerController _returnvalue))
  (bind _returnvalue_2 (UserInterface|CreateWidget "/Game/UserInterfaces/WB_MainMenu.WB_MainMenu_C" _asplayer_controller))
  (bind _output_get (Variables|Default|SetMainMenuWidget _returnvalue_2))
  (EventDispatchers|BindEventtoOnClickPlay _output_get (delegate Custom|StartPlayAnimation))
  (UserInterface|Viewport|AddtoViewport _returnvalue_2 0)
  (Variables|/Script/Engine.PlayerController|SetbShowMouseCursor _asplayer_controller true)
  (EventDispatchers|BindEventtoOnFinished (Variables|/Script/LevelSequence.LevelSequenceActor|GetSequencePlayer (Variables|Default|GetIntroSequencer)) (delegate Custom|OnFinishPlayAnimation)))

(fn ConstructionScript)