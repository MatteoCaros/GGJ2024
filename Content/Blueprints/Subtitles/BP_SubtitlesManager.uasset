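; Subtitle manager actor that plays queued voice clips with timed, speaker-colored subtitles from DT_Subtitles.
; On BeginPlay it creates the subtitle widget and hands itself to all I_AudioAndSubtitlesPlayer actors.
; AddAudioToPlay queues row names; PlayAudio loads each clip, stretching single-line subtitles to clip length.
; Tick advances lines by timestamp, plays a random funny sound between clips, and stops when the queue empties.
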(event EventTick
  (params (DeltaSeconds :type Float%20%28single-precision%29))
  (bind _linestoshow (Variables|Default|GetLinesToShow))
  (bind _output (Utilities|Array|Get(acopy) _linestoshow))
  (Variables|Default|SetActualClipTime (+ DeltaSeconds (Variables|Default|GetActualClipTime)))
  (bind _hasended_ (Default|FuncTickTimer (Variables|Default|GetSubtitlesWidget) DeltaSeconds))
  (if _hasended_
    (if (Utilities|Array|IsNotEmpty _linestoshow)
      (Default|ShowSubtitlesforTime (Variables|Default|GetSubtitlesWidget) (- (.timestamp _output) (Variables|Default|GetActualClipTime)) (Variables|Default|GetSpeaker) (.text _output) (Variables|Default|GetSpeakerColor))
      (Utilities|Array|RemoveIndex (Variables|Default|GetLinesToShow))
      (if (> (- (Variables|Default|GetInitialLinesToShow) (Utilities|Array|Length (Variables|Default|GetLinesToShow))) 1)
        (Utilities|FlowControl|DoOnce false :!label _label
          (:Completed
            (Default|ShowSecondText (Variables|Default|GetSubtitlesWidget)))))
      (else
        (Utilities|Array|RemoveIndex (Variables|Default|GetAudioToPlay))
        (Default|OnEndFullAudio (Variables|Default|GetSubtitlesWidget))
        (bind _alllinesended_ (CallFunction|PlayAudio))
        (Audio|PlaySound2D (.OutItem (Utilities|Array|Random (Variables|Default|GetFunnySounds))) 1.0 1.0 0.0 0 0)
        (if _alllinesended_
          (Actor|Tick|SetActorTickEnabled false)
          (Development|PrintString "Ended all clips  to play!")
          (Default|CallOnEndReadAlllines)
          (goto _label Reset))))))

(event EventBeginPlay
  (bind _outactors (Actor|GetAllActorsOfClass "/Game/Blueprints/BP_MainCharacter.BP_MainCharacter_C"))
  (Variables|Default|SetPlayerRef (Utilities|Array|Get(acopy) _outactors))
  (bind _returnvalue (UserInterface|CreateWidget "/Game/UserInterfaces/WB_Subtitles.WB_Subtitles_C" (.AsPlayer%20Controller (Utilities|Casting|CastToPlayerController (Pawn|GetController (Variables|Default|GetPlayerRef))))))
  (bind _output_get (Variables|Default|SetSubtitlesWidget _returnvalue))
  (UserInterface|Viewport|AddtoViewport _output_get 0)
  (bind _outactors_2 (Actor|GetAllActorswithInterface "/Game/Blueprints/Interfaces/I_AudioAndSubtitlesPlayer.I_AudioAndSubtitlesPlayer_C"))
  (for _array_element _outactors_2
    (Class|IAudioandSubtitlesPlayer|SetSubtitlesManagerRef(Message) _array_element self)))

(fn ConstructionScript)

(fn PlayAudio
  (bind _audiotoplay (Variables|Default|GetAudioToPlay))
  (bind _output (Utilities|Array|Get(acopy) _audiotoplay))
  (if (Utilities|Array|IsNotEmpty _audiotoplay)
    (Variables|Default|SetActualClipTime 0.0)
    (bind _returnvalue (Utilities|GetDataTableRow "/Game/Other/DataTables/DT_Subtitles.DT_Subtitles" _output)
      (:then
        (Variables|Default|SetSpeaker (.speakername _returnvalue))
        (Variables|Default|SetSpeakerColor (.speakertextcolor _returnvalue))
        (Audio|Components|Audio|SetSound (Variables|Default|GetAudio) (.audioclip _returnvalue))
        (bind _output_get (Variables|Default|SetLinesToShow (.timestamps _returnvalue)))
        (if (== (Utilities|Array|Length _output_get) 1)
          (Utilities|Array|SetArrayElem (Variables|Default|GetLinesToShow) 0 (Utilities|Struct|MakeS_TimeStampToText (Variables|/Script/Engine.SoundBase|GetDuration (.audioclip _returnvalue)) (.text (Utilities|Array|Get(acopy) (Variables|Default|GetLinesToShow))))))
        (Audio|Components|Audio|Play (Variables|Default|GetAudio) 0.0)
        (Actor|Tick|SetActorTickEnabled true)
        (Variables|Default|SetInitialLinesToShow (Utilities|Array|Length (Variables|Default|GetLinesToShow)))
        (return false))
      (:RowNotFound
        ;[1 1 1] Try next audio
        (Development|PrintString (Utilities|String|Append "NOT FOUNDED " (Utilities|String|ToString(Name) _output) " CLIP"))
        (Utilities|Array|RemoveIndex (Variables|Default|GetAudioToPlay))
        (CallFunction|PlayAudio)))
    (else
      (return true))))

(fn AddAudiotoPlay
  (params (AudioRowName :type Name))
  (bind _audiotoplay (Variables|Default|GetAudioToPlay))
  (Utilities|Array|Add _audiotoplay AudioRowName)
  (if (== (Utilities|Array|Length _audiotoplay) 1)
    (CallFunction|PlayAudio)))