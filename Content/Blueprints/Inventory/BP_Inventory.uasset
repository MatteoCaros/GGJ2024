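; BP_Inventory lets the player look at pickup items, see their names, and collect them into an inventory.
; Each tick, a sphere trace from the connected actor's first-person camera finds BP_MasterPickUpItem actors and updates the name and notification widget.
; When the interact input completes, it reuses that trace hit to store the item data in a map keyed by name, shows a notification, and destroys the actor.
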(event Input|EnhancedActionEvents|EnhancedInputActionIA_Interact
  (params (ActionValue :type Boolean) (ElapsedSeconds :type Float%20%28double-precision%29) (TriggeredSeconds :type Float%20%28double-precision%29) (InputAction :type Input%20Action%20Object%20Reference :default "/Game/Inputs/Actions/IA_Interact.IA_Interact"))
  (bind _item_name (Variables|Default|GetItem_Name))
  (:Completed
    (bind _added_ (CallFunction|TryAddItem (.HitActor (Collision|BreakHitResult (stale EventTick _outhit)))))
    (if _added_
      (bind _asbp_master_pick_up_item (Utilities|Casting|CastToBP_MasterPickUpItem (.HitActor (Collision|BreakHitResult (stale EventTick _outhit)))))
      (Default|SetNotifyItem _item_name (.name (Variables|/Game/Blueprints/Inventory/BP_MasterPickUpItem.BP_MasterPickUpItem_C|GetItemData _asbp_master_pick_up_item)))
      (Actor|DestroyActor (.HitActor (Collision|BreakHitResult (stale EventTick _outhit))))
      (Default|ResetLookItem _item_name))))

(event EventTick
  (params (DeltaSeconds :type Float%20%28single-precision%29))
  (bind _connectedactor (Variables|Default|GetConnectedActor))
  (bind _item_name (Variables|Default|GetItem_Name))
  (bind _firstpersoncamera (Variables|/Game/Blueprints/BP_MainCharacter.BP_MainCharacter_C|GetFirstPersonCamera _connectedactor))
  (bind _returnvalue (Transformation|GetWorldLocation _firstpersoncamera))
  (bind (_outhit _returnvalue_2) (Collision|SphereTraceByChannel _returnvalue (+ _returnvalue (* (Math|Vector|GetForwardVector _firstpersoncamera) (Variables|Default|GetInteractionRange))) 3e+01 "TraceTypeQuery1" false 0 "None"))
  (if _returnvalue_2
    (bind _asbp_master_pick_up_item (Utilities|Casting|CastToBP_MasterPickUpItem (.HitActor (Collision|BreakHitResult _outhit))))
    (Default|SetLookItem _item_name (.name (Variables|/Game/Blueprints/Inventory/BP_MasterPickUpItem.BP_MasterPickUpItem_C|GetItemData _asbp_master_pick_up_item)))
    (else
      (Default|ResetLookItem _item_name))))

(event EventBeginPlay
  (bind _returnvalue (UserInterface|CreateWidget "/Game/UserInterfaces/WB_ItemViewNameAndNotification.WB_ItemViewNameAndNotification_C"))
  (bind _output_get (Variables|Default|SetItem_Name _returnvalue))
  (UserInterface|Viewport|AddtoViewport _output_get 0))

(fn TryAddItem
  (params (HitActor :type Actor%20Object%20Reference))
  (bind _asbp_master_pick_up_item (Utilities|Casting|CastToBP_MasterPickUpItem HitActor)
    (:then
      (LocalVariables|SetCurrentItem (Variables|/Game/Blueprints/Inventory/BP_MasterPickUpItem.BP_MasterPickUpItem_C|GetItemData _asbp_master_pick_up_item))
      (CallFunction|AddItemtoInventory (LocalVariables|GetCurrentItem))
      (Development|PrintString (Utilities|String|Append (.Name (Utilities|Struct|BreakS_ItemData (LocalVariables|GetCurrentItem))) " Added to inventory!"))
      (return true))
    (:CastFailed
      (LocalVariables|SetCurrentItem "")
      (return false))))

(fn AddItemtoInventory
  (params (Item :type S%20Item%20Data%20Structure))
  (Utilities|Map|Add (Variables|Default|GetInventory) (.Name (Utilities|Struct|BreakS_ItemData Item)) Item))